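; BP_Target is a moving shootable target that loses health when hit by a first-person projectile.
; The construction script gives its InterpToMovement two relative control points: the actor's origin and MoveToPos.
; Non-lethal hits push Health into the HealthBar widget and show it until a delay hides it.
; At zero health it increments the player character's TargetsHit, calls CheckGoal and destroys itself.
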(event EventBeginPlay
  (CallFunction|UpdateHealthBar))

(event Collision|EventHit
  (params (MyComp :type Primitive%20Component%20Object%20Reference) (Other :type Actor%20Object%20Reference) (OtherComp :type Primitive%20Component%20Object%20Reference) (bSelfMoved :type Boolean) (HitLocation :type Vector :default "0, 0, 0") (HitNormal :type Vector :default "0, 0, 0") (NormalImpulse :type Vector :default "0, 0, 0") (Hit :type Hit%20Result%20Structure%20%28by%20ref%29))
  (Utilities|Casting|CastToBP_FirstPersonProjectile Other)
  (bind _output_get (Variables|Default|SetHealth (- (Variables|Default|GetHealth) 25.0)))
  (if (<= _output_get 0)
    (bind _asbp_first_person_character (Utilities|Casting|CastToBP_FirstPersonCharacter (Game|GetPlayerCharacter 0)))
    (Math|Integer|IncrementInt (Variables|/Game/FirstPerson/Blueprints/BP_FirstPersonCharacter.BP_FirstPersonCharacter_C|GetTargetsHit _asbp_first_person_character)
      (:%20%20
        (Default|CheckGoal _asbp_first_person_character)
        (Actor|DestroyActor)))
    (else
      (CallFunction|UpdateHealthBar)
      (Rendering|SetVisibility (Variables|Default|GetHealthBar) true false)
      (Utilities|FlowControl|Delay 5.0)
      (Rendering|SetVisibility (Variables|Default|GetHealthBar) false false))))

(fn ConstructionScript
  ;[1 1 1] Move Actor To Position
  (Class|InterptoMovementComponent|AddControlPointPosition (Variables|Components|GetInterpToMovement) "0, 0, 0" true)
  (Class|InterptoMovementComponent|AddControlPointPosition (Variables|Components|GetInterpToMovement) (Variables|Default|GetMoveToPos) true))

(fn UpdateHealthBar
  (bind _ashealth_bar (Utilities|Casting|CastToHealthBar (UserInterface|GetUserWidgetObject (Variables|Default|GetHealthBar))))
  (Variables|/Game/UI/HealthBar.HealthBar_C|SetHealth _ashealth_bar (Variables|Default|GetHealth))
  (return))